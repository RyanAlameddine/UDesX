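; Player controller that streams a grid of VoxelActor chunks around the player's pawn.
; Each tick it updates the pawn's chunk indices, spawns missing chunks within RenderRange and destroys those failing CheckRadius, tracked in parallel coordinate and actor arrays.
; Chunk indices divide position by half the chunk size, while placement uses the full size.
; CheckRadius holds only an unconnected distance test, and removal deletes array entries during forward iteration.
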(event `self.ReceiveBeginPlay`
  (`self.initialize`))

(event `self.ReceiveTick`
  (params (DeltaSeconds :type "Float (single-precision)"))
  (`self.updatePosition`)
  (`self.addChunk`)
  (`self.removeChunks`))

(fn `addChunk`
  (bind _renderrange (`self.renderRange`))
  (bind _chunkcoords (`self.chunkCoords`))
  (bind _returnvalue (`KismetMathLibrary.Conv_IntToDouble` (`self.chunkSize`)))
  (bind _returnvalue_2 (`KismetMathLibrary.Conv_IntToDouble` (`self.chunkSizeHalf`)))
  (bind _returnvalue_3 (* _renderrange -1))
  (for _index (range _returnvalue_3 (+ _renderrange 1))
    (for _index_2 (range _returnvalue_3 (+ _renderrange 1))
      (bind _returnvalue_4 (+ _index (`self.chunkX`)))
      (bind _returnvalue_5 (* _returnvalue_4 _returnvalue))
      (bind _returnvalue_6 (+ _index_2 (`self.chunkY`)))
      (bind _returnvalue_7 (* _returnvalue_6 _returnvalue))
      (if (`self.checkRadius` (+ _returnvalue_5 _returnvalue_2) (+ _returnvalue_7 _returnvalue_2))
        (bind _returnvalue_8 (`KismetMathLibrary.Conv_IntToDouble` _returnvalue_4))
        (bind _returnvalue_9 (`KismetMathLibrary.Conv_IntToDouble` _returnvalue_6))
        (if (not (`KismetArrayLibrary.Array_Contains` _chunkcoords (`KismetMathLibrary.MakeVector2D` _returnvalue_8 _returnvalue_9)))
          (`KismetArrayLibrary.Array_Add` _chunkcoords (`KismetMathLibrary.MakeVector2D` _returnvalue_8 _returnvalue_9))
          (bind _returnvalue_10 (`|SpawnActorFromClass` "/Script/UDesX.VoxelActor" (`KismetMathLibrary.Conv_VectorToTransform` (`KismetMathLibrary.MakeVector` _returnvalue_5 _returnvalue_7)) "Undefined" "OverrideRootScale" null 0 100 10 _returnvalue_4 _returnvalue_6 null))
          (`KismetArrayLibrary.Array_Add` (`self.chunks`) _returnvalue_10))))))

(fn `initialize`
  (bind _output_get (set `self.chunkSize` (* (`self.chunkLineElements`) (`self.voxelSize`))))
  (set `self.chunkSizeHalf` (/ _output_get 2)))

(fn `removeChunks`
  (bind _chunksize (`self.chunkSize`))
  (bind _chunks (`self.chunks`))
  (bind _returnvalue (`KismetMathLibrary.Conv_IntToDouble` (`self.chunkSizeHalf`)))
  (for (_array_element _array_index) (`self.chunkCoords`)
    (bind (_x _y) (`KismetMathLibrary.BreakVector2D` _array_element))
    (if (not (`self.checkRadius` (+ _returnvalue (* _chunksize _x)) (+ _returnvalue (* _chunksize _y))))
      (`self.K2_DestroyActor` (`|GetArrayItem` _chunks _array_index))
      (`KismetArrayLibrary.Array_Remove` _chunks _array_index)
      (`KismetArrayLibrary.Array_Remove` (`self.chunkCoords`) _array_index))))

(fn `updatePosition`
  (returns (wasChanged :type Boolean))
  (bind _returnvalue (`KismetMathLibrary.Conv_IntToDouble` (`self.chunkSizeHalf`)))
  (bind _output_get (set `self.characterPosition` (* (`self.K2_GetActorLocation` (`GameplayStatics.GetPlayerPawn` 0)) (1.0 1.0 0.0))))
  (bind _returnvalue_2 (`KismetMathLibrary.FFloor` (/ (.x _output_get) _returnvalue)))
  (bind _returnvalue_3 (`KismetMathLibrary.FFloor` (/ (.y _output_get) _returnvalue)))
  (if (or (!= (`self.chunkX`) _returnvalue_2) (!= (`self.chunkY`) _returnvalue_3))
    (set `self.chunkX` _returnvalue_2)
    (set `self.chunkY` _returnvalue_3)
    (return true)
    (else
      (return false))))

(fn `UserConstructionScript`)